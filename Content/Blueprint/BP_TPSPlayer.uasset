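; Third-person shooter player character that connects input and state to screen, pause and game-over widgets.
; BeginPlay creates the HUD, then after a short delay fills in health and clears the grenade state, which drives the weapon display.
; Fire input calls an inherited-looking function, and overlapping BI_Unit actors receive OnMyHit with a large forward impulse vector.
; P opens the pause menu; game over calls the parent, then shows its screen.
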(event `self.ReceiveBeginPlay`
  (bind _returnvalue (`|CreateWidget` "/Game/Blueprint/WBP_ScreenUI.WBP_ScreenUI_C" (`GameplayStatics.GetPlayerController` 0)))
  (bind _output_get (set `self.uiScereen` _returnvalue))
  (`UserWidget.AddToViewport` _output_get 0)
  (`KismetSystemLibrary.Delay` 0.05)
  (`self.UIctrlHP`)
  (`self.OnUsingGrende` false))

(event `EnhancedInput|/Game/Input/IA_Fire`
  (params (ActionValue :type Boolean) (ElapsedSeconds :type "Float (double-precision)") (TriggeredSeconds :type "Float (double-precision)") (InputAction :type "InputAction Object Reference" :default "/Game/Input/IA_Fire.IA_Fire"))
  (:`Started`
    (`self.FCallName`)))

(event `EnhancedInput|/Game/Input/IA_Fire`
  (params (ActionValue :type Boolean) (ElapsedSeconds :type "Float (double-precision)") (TriggeredSeconds :type "Float (double-precision)") (InputAction :type "InputAction Object Reference" :default "/Game/Input/IA_Fire.IA_Fire")))

(event `self.ReceiveActorBeginOverlap`
  (params (OtherActor :type "Actor Object Reference"))
  (bind _asbi_unit (cast `/Game/InterfaceTest/BI_Unit` OtherActor))
  (`/Game/InterfaceTest/BI_Unit.OnMyHit` _asbi_unit (* (`self.GetActorForwardVector`) 500000.0)))

(event `self.ReceiveTick`
  (params (DeltaSeconds :type "Float (single-precision)")))

(event `self.OnUsingGrende`
  (params (isGrende :type Boolean))
  (bind _uiscereen (`self.uiScereen`))
  (`/Engine/EditorBlueprintResources/StandardMacros.IsValid` _uiscereen
    (:`Is Valid`
      (set `/Game/Blueprint/WBP_ScreenUI.isGrenaded` isGrende _uiscereen)
      (`/Game/Blueprint/WBP_ScreenUI.SwapWeapon` _uiscereen))))

(event `self.OnGameOver`
  (bind _returnvalue (`GameplayStatics.GetPlayerController` 0))
  (`parent.OnGameOver`)
  (set `PlayerController.bShowMouseCursor` true _returnvalue)
  (bind _returnvalue_2 (`|CreateWidget` "/Game/Blueprint/WBP_GameOver.WBP_GameOver_C" _returnvalue))
  (`UserWidget.AddToViewport` _returnvalue_2 0))

(event `Key|P`
  (params (Key :type "Key Structure"))
  (bind _returnvalue (`GameplayStatics.GetPlayerController` 0))
  (:`Pressed`
    (bind _returnvalue_2 (`|CreateWidget` "/Game/Blueprint/WBP_PauseMenu.WBP_PauseMenu_C"))
    (`UserWidget.AddToViewport` _returnvalue_2 0)
    (`GameplayStatics.SetGamePaused` true)
    (`WidgetBlueprintLibrary.SetInputMode_UIOnlyEx` _returnvalue null)
    (set `PlayerController.bShowMouseCursor` true _returnvalue)))

(fn `UIctrlHP`
  (set `/Game/Blueprint/WBP_ScreenUI.hpRatio` (/ (`KismetMathLibrary.Conv_IntToDouble` (`self.hp`)) (`KismetMathLibrary.Conv_IntToDouble` (`self.initialHp`))) (`self.uiScereen`))
  (set `/Game/Blueprint/WBP_ScreenUI.hpString` (`KismetStringLibrary.Concat_StrStr` (`KismetStringLibrary.Conv_IntToString` (`self.hp`)) "/" (`KismetStringLibrary.Conv_IntToString` (`self.initialHp`))) (`self.uiScereen`)))

(fn `UserConstructionScript`)