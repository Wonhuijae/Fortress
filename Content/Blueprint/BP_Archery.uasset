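; BP_Archery runs the archery game's screen UI, pause and game-over menus, and countdown timer.
; BeginPlay creates the HUD, then after a brief delay HPUICtrl pushes HP ratio and text to it once.
; P pauses into a UI-only menu, and OnGameOver calls the parent before showing its widget.
; A Delay on Tick steps minutes and seconds down each second; seconds still wrap to 59 at zero minutes, without triggering game over.
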(event `self.OnGameOver`
  (bind _returnvalue (`GameplayStatics.GetPlayerController` 0))
  ;[1 1 1] 게임오버시 GameOver UI 나타나게 하기
  (`parent.OnGameOver`)
  (set `PlayerController.bShowMouseCursor` true _returnvalue)
  (bind _returnvalue_2 (`|CreateWidget` "/Game/Blueprint/WBP_GameOver.WBP_GameOver_C" _returnvalue))
  (`UserWidget.AddToViewport` _returnvalue_2 0))

(event `Key|P`
  (params (Key :type "Key Structure"))
  (bind _returnvalue (`GameplayStatics.GetPlayerController` 0))
  ;[1 1 1] 키보드의 p를 누르면 pause UI 나타나게 함
  (:`Pressed`
    (`GameplayStatics.SetGamePaused` true)
    (bind _returnvalue_2 (`|CreateWidget` "/Game/Blueprint/WBP_PauseMenu.WBP_PauseMenu_C"))
    (`UserWidget.AddToViewport` _returnvalue_2 0)
    (`WidgetBlueprintLibrary.SetInputMode_UIOnlyEx` _returnvalue null)
    (set `PlayerController.bShowMouseCursor` true _returnvalue)))

(event `self.ReceiveBeginPlay`
  ;[1 1 1] 게임이 시작하면 기본적인 게임 UI가 나타나게 함
  (bind _returnvalue (`|CreateWidget` "/Game/Blueprint/WBP_ScreenUI_Archery.WBP_ScreenUI_Archery_C" (`GameplayStatics.GetPlayerController` 0)))
  (bind _output_get (set `self.ArcheryUIScreen` _returnvalue))
  (`UserWidget.AddToViewport` _output_get 0)
  (`KismetSystemLibrary.Delay` 0.005)
  (`self.HPUICtrl`))

(event `self.ReceiveTick`
  (params (DeltaSeconds :type "Float (single-precision)"))
  ;[1 1 1] 시간이 줄어드는 타이머 만들기
  (`KismetSystemLibrary.Delay` 1.0)
  (if (== (`self.Seconds_A`) 0)
    (`|ExecutionSequence`
      (:`then_0`
        ;;[1 1 1] 0초가 맞고, 0분이 아닐경우, 초는 다시 59초로 세팅되고, 0분이 될 때까지 1분씩 차감
        (if (not (== (`self.Minutes_A`) 0))
          (set `self.Seconds_A` 59)
          (set `self.Minutes_A` (- (`self.Minutes_A`) 1))))
      (:`then_1`
        ;;[1 1 1] 0초가 맞는 경우, 다시 59초로 리셋
        (set `self.Seconds_A` 59)))
    (else
      ;;[1 1 1] 0초가 아닐 경우, 0초가 될때까지 1초씩 차감
      (set `self.Seconds_A` (- (`self.Seconds_A`) 1)))))

(fn `HPUICtrl`
  (set `/Game/Blueprint/WBP_ScreenUI_Archery.hpRatio` (/ (`self.hp`) (`self.maxHp`)) (`self.ArcheryUIScreen`))
  (set `/Game/Blueprint/WBP_ScreenUI_Archery.hpString` (`KismetStringLibrary.Concat_StrStr` (`KismetStringLibrary.Conv_IntToString` (`self.hp`)) "/" (`KismetStringLibrary.Conv_IntToString` (`self.maxHp`))) (`self.ArcheryUIScreen`)))

(fn `UserConstructionScript`)